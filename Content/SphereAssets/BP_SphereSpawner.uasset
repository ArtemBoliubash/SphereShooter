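; BP_SphereSpawner spawns waves of spheres as existing ones are destroyed.
; On BeginPlay it binds a handler to changes in the destroyed-sphere count.
; When that count exceeds the wave threshold, it calls SpawnSpheres with fixed increases to sphere number and radius.
; It then resets the count and raises the threshold by ten percent, so each following wave requires more destroyed spheres.
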(event `self.ReceiveBeginPlay`
  (add `self.OnQuantityDestroyedSpheresChange` (delegate `OnDestroyedSphere`)))

(event `OnDestroyedSphere`
  (if (> (`self.QuantityDestroyedSpheres`) (`self.NewWaveQuantity`))
    (`self.SpawnSpheres` 10 5)
    (set `self.QuantityDestroyedSpheres` 0)
    (set `self.NewWaveQuantity` (+ (`self.NewWaveQuantity`) (/ (* (`self.NewWaveQuantity`) 10) 100)))))

(fn `UserConstructionScript`)